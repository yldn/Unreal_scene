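; Japanese-themed hologram actor that the player toggles on and off with the 7 key.
; A FlipFlop starts or stops the NSCityRay effect and plays one of two timelines that drive dissolve and opacity on the two static meshes and the Ray.
; The construction script pushes color and rotation-speed variables into the materials and Niagara system.
; Tick feeds the NSCityRay world location to the Ray material's Point Location parameter.
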(event `self.ReceiveBeginPlay`
  (`self.EnableInput` (`GameplayStatics.GetPlayerController` 0)))

(event `Key|Seven`
  (params (Key :type "Key Structure"))
  (bind _staticmesh2 (`self.StaticMesh2`))
  (bind _staticmesh (`self.StaticMesh`))
  (:`Pressed`
    (`/Engine/EditorBlueprintResources/StandardMacros.FlipFlop`
      (:`A`
        (`ActorComponent.SetActive` (`self.NS_City_Ray`) true false)
        (bind (_direction _dissolve) (`Timeline|Timeline` :!via `PlayFromStart`)
          (:`Update`
            (`MeshComponent.SetScalarParameterValueOnMaterials` _staticmesh2 "opacity_all" 0.6)
            (`MeshComponent.SetScalarParameterValueOnMaterials` _staticmesh2 "Dissolve" _dissolve)
            (`MeshComponent.SetScalarParameterValueOnMaterials` _staticmesh "opacity_all" 0.6)
            (`MeshComponent.SetScalarParameterValueOnMaterials` _staticmesh "Dissolve" _dissolve)
            (`MeshComponent.SetScalarParameterValueOnMaterials` (`self.Ray`) "opacity_all" 0.12))))
      (:`B`
        (`ActorComponent.Deactivate` (`self.NS_City_Ray`))
        (bind (_direction_2 _dissolve_2 _opacity) (`Timeline|Timeline_1` :!via `PlayFromStart`)
          (:`Update`
            (`MeshComponent.SetScalarParameterValueOnMaterials` (`self.StaticMesh`) "Dissolve" _dissolve_2)
            (`MeshComponent.SetScalarParameterValueOnMaterials` (`self.StaticMesh2`) "Dissolve" _dissolve_2)
            (`MeshComponent.SetScalarParameterValueOnMaterials` (`self.Ray`) "opacity_all" (* _opacity 0.25))
            (`MeshComponent.SetScalarParameterValueOnMaterials` (`self.StaticMesh`) "opacity_all" _opacity)))))))

(event `self.ReceiveTick`
  (params (DeltaSeconds :type "Float (single-precision)"))
  (`MeshComponent.SetVectorParameterValueOnMaterials` (`self.Ray`) "Point Location" (`SceneComponent.K2_GetComponentLocation` (`self.NS_City_Ray`))))

(fn `UserConstructionScript`
  (bind _ray (`self.Ray`))
  (bind _returnvalue (`KismetMathLibrary.Conv_LinearColorToVector` (`self.Color`)))
  (`MeshComponent.SetVectorParameterValueOnMaterials` (`self.StaticMesh`) "Color" (`KismetMathLibrary.Conv_LinearColorToVector` (`self.Color_0`)))
  (`MeshComponent.SetVectorParameterValueOnMaterials` _ray "Color" _returnvalue)
  (`MeshComponent.SetVectorParameterValueOnMaterials` (`self.StaticMesh2`) "Color" _returnvalue)
  (`NiagaraComponent.SetVariableLinearColor` (`self.NS_City_Ray`) "Color" (`KismetMathLibrary.Conv_VectorToLinearColor` _returnvalue))
  (`MeshComponent.SetVectorParameterValueOnMaterials` _ray "Point Location" (`SceneComponent.K2_GetComponentLocation` (`self.NS_City_Ray`)))
  (`MeshComponent.SetScalarParameterValueOnMaterials` (`self.StaticMesh`) "rotate speed" (`self.Rotate Speed`))
  (`MeshComponent.SetScalarParameterValueOnMaterials` (`self.StaticMesh2`) "rotate speed" (`self.Rotate Speed2`)))