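; Hologram display actor that endlessly cycles its static mesh through brain, cube and heart models on two-second delays from BeginPlay.
; Key 3 flip-flops the projection: it activates or deactivates the NSSMRay Niagara effect while timelines drive dissolve and opacity material parameters on mesh and ray.
; The construction script applies one Color to mesh, ray and particles, and Tick feeds the effect's world location into the ray material.
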(event `Play Again`
  (bind _staticmesh (`self.StaticMesh`))
  (`StaticMeshComponent.SetStaticMesh` _staticmesh "/Game/Hologram/Resource/Mesh/SM_Brain_M.SM_Brain_M" :!label _label)
  (`KismetSystemLibrary.Delay` 2.0)
  (`StaticMeshComponent.SetStaticMesh` _staticmesh "/Game/Hologram/Resource/Mesh/SM_Cube.SM_Cube")
  (`KismetSystemLibrary.Delay` 2.0)
  (`StaticMeshComponent.SetStaticMesh` _staticmesh "/Game/Hologram/Resource/Mesh/SM_Heart_M.SM_Heart_M")
  (`KismetSystemLibrary.Delay` 2.0)
  (`self.Play Again`))

(event `self.ReceiveBeginPlay`
  (`self.EnableInput` (`GameplayStatics.GetPlayerController` 0))
  (goto _label))

(event `Key|Three`
  (params (Key :type "Key Structure"))
  (bind _staticmesh (`self.StaticMesh`))
  (bind _ns_sm_ray (`self.NS_SM_Ray`))
  (:`Pressed`
    (`/Engine/EditorBlueprintResources/StandardMacros.FlipFlop`
      (:`A`
        (`ActorComponent.SetActive` _ns_sm_ray true false)
        (bind (_direction _dissolve) (`Timeline|Timeline` :!via `PlayFromStart`)
          (:`Update`
            (`MeshComponent.SetScalarParameterValueOnMaterials` _staticmesh "opacity_all" 0.6)
            (`MeshComponent.SetScalarParameterValueOnMaterials` _staticmesh "Dissolve" _dissolve)
            (`MeshComponent.SetScalarParameterValueOnMaterials` (`self.Ray`) "opacity_all" 0.12))))
      (:`B`
        (`ActorComponent.Deactivate` _ns_sm_ray)
        (bind (_direction_2 _dissolve_2 _opacity) (`Timeline|Timeline_1` :!via `PlayFromStart`)
          (:`Update`
            (`MeshComponent.SetScalarParameterValueOnMaterials` (`self.StaticMesh`) "Dissolve" _dissolve_2)
            (`MeshComponent.SetScalarParameterValueOnMaterials` (`self.Ray`) "opacity_all" (* _opacity 0.25))
            (`MeshComponent.SetScalarParameterValueOnMaterials` (`self.StaticMesh`) "opacity_all" _opacity)))))))

(event `self.ReceiveTick`
  (params (DeltaSeconds :type "Float (single-precision)"))
  (`MeshComponent.SetVectorParameterValueOnMaterials` (`self.Ray`) "Point Location" (`SceneComponent.K2_GetComponentLocation` (`self.NS_SM_Ray`))))

(fn `UserConstructionScript`
  (bind _ns_sm_ray (`self.NS_SM_Ray`))
  (bind _ray (`self.Ray`))
  (bind _returnvalue (`KismetMathLibrary.Conv_LinearColorToVector` (`self.Color`)))
  (`MeshComponent.SetVectorParameterValueOnMaterials` (`self.StaticMesh`) "Color" _returnvalue)
  (`MeshComponent.SetVectorParameterValueOnMaterials` _ray "Color" _returnvalue)
  (`MeshComponent.SetVectorParameterValueOnMaterials` _ray "Point Location" (`SceneComponent.K2_GetComponentLocation` _ns_sm_ray))
  (`NiagaraComponent.SetVariableLinearColor` _ns_sm_ray "Color" (`KismetMathLibrary.Conv_VectorToLinearColor` _returnvalue)))