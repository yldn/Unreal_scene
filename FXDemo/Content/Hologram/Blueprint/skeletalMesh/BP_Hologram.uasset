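; Hologram actor that shows a running skeletal mesh with a dissolve effect and a ray whose material tracks a point in the world.
; BeginPlay loops the run animation and starts the Dissolve timeline, which the playagain event can restart.
; The timeline writes its value to both a material scalar and custom primitive data on the mesh.
; Construction and Tick feed RayLocation's world position into the Ray material's Point Location parameter.
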(event `play again`
  (bind _skeletalmesh (`self.SkeletalMesh`))
  (bind (_direction _dissolve) (`Timeline|Dissolve` :!via `PlayFromStart` :!label _label)
    (:`Update`
      (`MeshComponent.SetScalarParameterValueOnMaterials` _skeletalmesh "Dissolve" _dissolve)
      (`PrimitiveComponent.SetCustomPrimitiveDataFloat` _skeletalmesh 0 _dissolve))))

(event `self.ReceiveBeginPlay`
  (`SkeletalMeshComponent.PlayAnimation` (`self.SkeletalMesh`) "/Game/Hologram/Demo/ThirdPerson/Characters/Mannequins/Animations/Manny/MM_Run_Fwd.MM_Run_Fwd" true)
  (goto _label :!via `PlayFromStart`))

(event `self.ReceiveTick`
  (params (DeltaSeconds :type "Float (single-precision)"))
  (`MeshComponent.SetVectorParameterValueOnMaterials` (`self.Ray`) "Point Location" (`SceneComponent.K2_GetComponentLocation` (`self.RayLocation`))))

(fn `UserConstructionScript`
  (`MeshComponent.SetVectorParameterValueOnMaterials` (`self.Ray`) "Point Location" (`SceneComponent.K2_GetComponentLocation` (`self.RayLocation`))))