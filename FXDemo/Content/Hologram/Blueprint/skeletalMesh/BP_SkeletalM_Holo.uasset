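; Hologram actor showing a looping run-animated skeletal mesh with a ray mesh and Niagara ray effect.
; Key 9 flip-flops the hologram: it toggles the Niagara effect and plays one of two timelines driving material dissolve and opacity on the meshes.
; The construction script applies one Color to both meshes and the effect.
; The ray mesh's material receives the effect's world location at construction and every Tick as its point location.
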(event `self.ReceiveBeginPlay`
  (`self.EnableInput` (`GameplayStatics.GetPlayerController` 0))
  (`SkeletalMeshComponent.PlayAnimation` (`self.SkeletalMesh`) "/Game/Hologram/Demo/ThirdPerson/Characters/Mannequins/Animations/Manny/MM_Run_Fwd.MM_Run_Fwd" true))

(event `Key|Nine`
  (params (Key :type "Key Structure"))
  (bind _skeletalmesh (`self.SkeletalMesh`))
  (bind _skeletalmesh_2 (`self.SkeletalMesh`))
  (:`Pressed`
    (`/Engine/EditorBlueprintResources/StandardMacros.FlipFlop`
      (:`A`
        (`ActorComponent.SetActive` (`self.NS_Skeletal_Ray`) true false)
        (bind (_direction _dissolve) (`Timeline|Timeline` :!via `PlayFromStart`)
          (:`Update`
            (`MeshComponent.SetScalarParameterValueOnMaterials` _skeletalmesh_2 "opacity_all" 0.6)
            (`MeshComponent.SetScalarParameterValueOnMaterials` _skeletalmesh_2 "Dissolve" _dissolve)
            (`MeshComponent.SetScalarParameterValueOnMaterials` (`self.SkeletalMesh_Ray`) "opacity_all" 0.12))))
      (:`B`
        (`ActorComponent.Deactivate` (`self.NS_Skeletal_Ray`))
        (bind (_direction_2 _dissolve_2 _opacity) (`Timeline|Timeline_1` :!via `PlayFromStart`)
          (:`Update`
            (`MeshComponent.SetScalarParameterValueOnMaterials` _skeletalmesh "Dissolve" _dissolve_2)
            (`MeshComponent.SetScalarParameterValueOnMaterials` (`self.SkeletalMesh_Ray`) "opacity_all" (* _opacity 0.25))
            (`MeshComponent.SetScalarParameterValueOnMaterials` _skeletalmesh "opacity_all" _opacity)))))))

(event `self.ReceiveTick`
  (params (DeltaSeconds :type "Float (single-precision)"))
  (`MeshComponent.SetVectorParameterValueOnMaterials` (`self.SkeletalMesh_Ray`) "Point Location" (`SceneComponent.K2_GetComponentLocation` (`self.NS_Skeletal_Ray`))))

(fn `UserConstructionScript`
  (bind _skeletalmesh_ray (`self.SkeletalMesh_Ray`))
  (bind _returnvalue (`KismetMathLibrary.Conv_LinearColorToVector` (`self.Color`)))
  (`MeshComponent.SetVectorParameterValueOnMaterials` (`self.SkeletalMesh`) "Color" _returnvalue)
  (`MeshComponent.SetVectorParameterValueOnMaterials` _skeletalmesh_ray "Color" _returnvalue)
  (`NiagaraComponent.SetVariableLinearColor` (`self.NS_Skeletal_Ray`) "Color" (`KismetMathLibrary.Conv_VectorToLinearColor` _returnvalue))
  (`MeshComponent.SetVectorParameterValueOnMaterials` _skeletalmesh_ray "Point Location" (`SceneComponent.K2_GetComponentLocation` (`self.NS_Skeletal_Ray`))))