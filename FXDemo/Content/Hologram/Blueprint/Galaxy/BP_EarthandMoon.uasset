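; Hologram actor of the Earth and Moon, with projection rays and Niagara effects, toggled on and off by the 0 key.
; A FlipFlop activates or deactivates effects and plays timelines driving Earth dissolve and material opacity, animating opacity only when switching off.
; The construction script applies a shared color and aims each ray material at its Niagara component's location.
; Tick refreshes that point only for the first ray.
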(event `self.ReceiveBeginPlay`
  (`self.EnableInput` (`GameplayStatics.GetPlayerController` 0)))

(event `Key|Zero`
  (params (Key :type "Key Structure"))
  (bind _ns_ray_location2 (`self.NS_Ray_Location2`))
  (bind _ray2 (`self.Ray2`))
  (bind _ns_earthmoon (`self.NS_EarthMoon`))
  (bind _ray1 (`self.Ray1`))
  (bind _earth (`self.Earth`))
  (bind _ns_ray_location1 (`self.NS_Ray_Location1`))
  (:`Pressed`
    (`/Engine/EditorBlueprintResources/StandardMacros.FlipFlop`
      (:`A`
        (`ActorComponent.SetActive` (`self.NS_Ray_Location`) true false)
        (`ActorComponent.SetActive` _ns_ray_location1 true false)
        (`ActorComponent.SetActive` _ns_ray_location2 true false)
        (`ActorComponent.SetActive` _ray2 true false)
        (`ActorComponent.SetActive` _ns_earthmoon true false)
        (`ActorComponent.SetActive` _ray1 true false)
        (bind (_direction _dissolve) (`Timeline|Timeline` :!via `PlayFromStart`)
          (:`Update`
            (`MeshComponent.SetScalarParameterValueOnMaterials` _earth "opacity_all" 0.6)
            (`MeshComponent.SetScalarParameterValueOnMaterials` _earth "Dissolve" _dissolve)
            (`MeshComponent.SetScalarParameterValueOnMaterials` (`self.Ray`) "opacity_all" 0.12)
            (`MeshComponent.SetScalarParameterValueOnMaterials` (`self.Ray1`) "opacity_all" 0.12)
            (`MeshComponent.SetScalarParameterValueOnMaterials` (`self.Ray2`) "opacity_all" 0.12))))
      (:`B`
        (`ActorComponent.Deactivate` (`self.NS_Ray_Location`))
        (`ActorComponent.Deactivate` _ns_ray_location1)
        (`ActorComponent.Deactivate` _ns_ray_location2)
        (`ActorComponent.Deactivate` _ray2)
        (`ActorComponent.Deactivate` _ns_earthmoon)
        (`ActorComponent.Deactivate` _ray1)
        (bind (_direction_2 _dissolve_2 _opacity) (`Timeline|Timeline_1` :!via `PlayFromStart`)
          (:`Update`
            (`MeshComponent.SetScalarParameterValueOnMaterials` (`self.Earth`) "Dissolve" _dissolve_2)
            (bind _returnvalue (* _opacity 0.25))
            (`MeshComponent.SetScalarParameterValueOnMaterials` (`self.Ray`) "opacity_all" _returnvalue)
            (`MeshComponent.SetScalarParameterValueOnMaterials` (`self.Earth`) "opacity_all" _opacity)
            (`MeshComponent.SetScalarParameterValueOnMaterials` (`self.Ray1`) "opacity_all" _returnvalue)
            (`MeshComponent.SetScalarParameterValueOnMaterials` (`self.Ray2`) "opacity_all" _returnvalue)))))))

(event `self.ReceiveTick`
  (params (DeltaSeconds :type "Float (single-precision)"))
  (`MeshComponent.SetVectorParameterValueOnMaterials` (`self.Ray`) "Point Location" (`SceneComponent.K2_GetComponentLocation` (`self.NS_Ray_Location`))))

(fn `UserConstructionScript`
  (bind _ray1 (`self.Ray1`))
  (bind _ray2 (`self.Ray2`))
  (bind _ray (`self.Ray`))
  (bind _returnvalue (`KismetMathLibrary.Conv_LinearColorToVector` (`self.Color`)))
  (bind _returnvalue_2 (`KismetMathLibrary.Conv_VectorToLinearColor` _returnvalue))
  (`MeshComponent.SetVectorParameterValueOnMaterials` (`self.Earth`) "Color" _returnvalue)
  (`NiagaraComponent.SetVariableLinearColor` (`self.NS_Ray_Location`) "Color" (`KismetMathLibrary.Conv_VectorToLinearColor` _returnvalue))
  (`MeshComponent.SetVectorParameterValueOnMaterials` _ray "Color" _returnvalue)
  (`MeshComponent.SetVectorParameterValueOnMaterials` _ray "Point Location" (`SceneComponent.K2_GetComponentLocation` (`self.NS_Ray_Location`)))
  (`MeshComponent.SetVectorParameterValueOnMaterials` _ray1 "Color" _returnvalue)
  (`MeshComponent.SetVectorParameterValueOnMaterials` _ray1 "Point Location" (`SceneComponent.K2_GetComponentLocation` (`self.NS_Ray_Location1`)))
  (`MeshComponent.SetVectorParameterValueOnMaterials` _ray2 "Color" _returnvalue)
  (`MeshComponent.SetVectorParameterValueOnMaterials` _ray2 "Point Location" (`SceneComponent.K2_GetComponentLocation` (`self.NS_Ray_Location2`)))
  (`NiagaraComponent.SetVariableLinearColor` (`self.NS_Ray_Location1`) "Color" _returnvalue_2)
  (`NiagaraComponent.SetVariableLinearColor` (`self.NS_Ray_Location2`) "Color" _returnvalue_2))